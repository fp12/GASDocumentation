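; GA_SelectiveArea is a GAS hero ability that applies GE_SelectiveArea_Target to nearby actors selected by name.
; On activation it commits, then runs an instant WaitTargetData with a radius target actor at the avatar, sized by AreaRadius.
; A custom GDNameTargetDataFilter narrows targets by NameFilter, case-sensitively, and excludes the avatar.
; Valid data applies the effect and ends the ability; an unused node shows the simpler helper for building the filter.
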(event `self.K2_ActivateAbility`
  (`self.K2_CommitAbility`)
  (bind (_asynctaskproxy _data) (`AbilityTask_WaitTargetData.WaitTargetData` "None" "Instant" "/Script/GameplayAbilities.GameplayAbilityTargetActor_Radius" (`self.AreaRadius`) (make `GameplayAbilityTargetingLocationInfo` "ActorTransform" "0.000000,0.000000,0.000000|0.000000,0.000000,0.000000|1.000000,1.000000,1.000000" (`self.GetAvatarActorFromActorInfo`)) (struct) null (`GDTargetDataFilterBlueprintLibrary.MakeGDNameFilterHandle` (make `GDNameTargetDataFilter` (`self.NameFilter`) true "TDFS_NoSelf") (`self.GetAvatarActorFromActorInfo`)))
    (:`ValidData`
      (`self.BP_ApplyGameplayEffectToTarget` _data "/Game/GASDocumentation/Characters/Hero/Abilities/SelectiveArea/GE_SelectiveArea_Target.GE_SelectiveArea_Target_C")
      (`self.K2_EndAbility`))
    (:`Cancelled`
      (`self.K2_EndAbility`))))